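; BP_RuneOrb is a collectible orb that grants a Sheikah rune, calling RunePickedUp with its SheikahRune value when picked up and then destroying itself.
; Each tick the static mesh bobs vertically around its starting relative position on a cosine of time since creation, scaled by speed and amplitude variables.
; The Paper sprite is billboarded on yaw only, turning toward the player camera while staying upright.
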(event `self.ReceiveBeginPlay`
  (bind _returnvalue_location (`KismetMathLibrary.BreakTransform` (`SceneComponent.GetRelativeTransform` (`self.StaticMesh`))))
  (set `self.StartingRelativePos` _returnvalue_location))

(event `self.PickUpObject`
  (`self.RunePickedUp` (`self.SheikahRune`))
  (`self.K2_DestroyActor`))

(event `self.ReceiveTick`
  (params (DeltaSeconds :type "Float (single-precision)"))
  (`SceneComponent.K2_SetWorldRotation` (`self.PaperSprite`) (`KismetMathLibrary.MakeRotator` 0.0 0.0 (+ (.yaw (`KismetMathLibrary.FindLookAtRotation` (`PlayerCameraManager.GetCameraLocation` (`GameplayStatics.GetPlayerCameraManager` 0)) (`SceneComponent.K2_GetComponentLocation` (`self.PaperSprite`)))) 90.0)) false false)
  (`SceneComponent.K2_SetRelativeLocation` (`self.StaticMesh`) (+ (`self.StartingRelativePos`) (`KismetMathLibrary.MakeVector` 0.0 0.0 (* (`KismetMathLibrary.Cos` (* (`self.GetGameTimeSinceCreation`) (`self.SinSpeed`))) (`self.SinAmplitude`)))) false false))

(fn `UserConstructionScript`
  (`parent.UserConstructionScript`))