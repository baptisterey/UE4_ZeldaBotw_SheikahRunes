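; BPA_RotateObject is an actor component for shrine objects that continuously spins its owning actor.
; Each tick, while IsRotating is set, it adds a local rotation from the RotateAxis vector scaled by RotateSpeed and frame delta time.
; OnSheikahFreezed and OnSheikahReleased events turn the rotation off and on, so the object stops while frozen by the Sheikah ability.
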(event `self.ReceiveTick`
  (params (DeltaSeconds :type "Float (single-precision)"))
  (bind (_returnvalue_x _returnvalue_y _returnvalue_z) (`KismetMathLibrary.BreakVector` (* (* (`self.RotateAxis`) (`self.RotateSpeed`)) (`GameplayStatics.GetWorldDeltaSeconds`))))
  (if (`self.IsRotating`)
    (`Actor.K2_AddActorLocalRotation` (`self.GetOwner`) (`KismetMathLibrary.MakeRotator` _returnvalue_x _returnvalue_y _returnvalue_z) false false)))

(event `/Game/Blueprints/CharacterLogic/SheikahRunes/Stasis/BPI_StasisInteraction.OnSheikahFreezed`
  (set `self.IsRotating` false))

(event `/Game/Blueprints/CharacterLogic/SheikahRunes/Stasis/BPI_StasisInteraction.OnSheikahReleased`
  (set `self.IsRotating` true))