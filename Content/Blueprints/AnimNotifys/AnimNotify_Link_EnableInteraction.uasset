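; Animation notify that toggles an interaction-related movement action on the character that owns the animated mesh.
; When fired, it casts the mesh owner to Character and sends it a movement action through a Blueprint Interface message, avoiding a dependency on a specific character class.
; The notify's IsInteracting flag selects which of two movement action enum values is sent.
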(fn `Received_Notify`
  (params (MeshComp :type "SkeletalMeshComponent Object Reference") (Animation :type "AnimSequenceBase Object Reference"))
  (returns (ReturnValue :type Boolean))
  (locals (LocalCharacter :type "Character Object Reference"))
  (bind _ascharacter (cast `Character` (`ActorComponent.GetOwner` MeshComp)))
  (set `local.LocalCharacter` _ascharacter)
  (if (not (`self.IsInteracting`))
    (message `/Game/AdvancedLocomotionV4/Blueprints/Interfaces/ALS_Character_BPI.BPI_Set_MovementAction` (`local.LocalCharacter`) "NewEnumerator4")
    (else
      (message `/Game/AdvancedLocomotionV4/Blueprints/Interfaces/ALS_Character_BPI.BPI_Set_MovementAction` (`local.LocalCharacter`) "NewEnumerator5")))
  (return false))