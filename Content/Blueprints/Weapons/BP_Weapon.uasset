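; BP_Weapon is a weapon actor that deals damage through hit box overlaps while attached to an owning actor.
; Its HitBoxes collision starts disabled on BeginPlay and is toggled between query-only and none by the SetCanDealDamage event.
; On overlap, it applies point damage using WeaponDamage and DamageType, with the attach parent as damage causer and a hit direction from that parent toward the overlapped actor.
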(event `self.ReceiveBeginPlay`
  (`self.SetCanDealDamage` false))

(event `SetCanDealDamage`
  (params (CanDealDamage :type Boolean))
  (if CanDealDamage
    (`PrimitiveComponent.SetCollisionEnabled` (`self.HitBoxes`) "QueryOnly")
    (else
      (`PrimitiveComponent.SetCollisionEnabled` (`self.HitBoxes`) "NoCollision"))))

(event `self.HitBoxes.OnComponentBeginOverlap`
  (params (OverlappedComponent :type "PrimitiveComponent Object Reference") (OtherActor :type "Actor Object Reference") (OtherComp :type "PrimitiveComponent Object Reference") (OtherBodyIndex :type Integer) (bFromSweep :type Boolean) (SweepResult :type "HitResult Structure (by ref)"))
  (bind _returnvalue (`self.GetAttachParentActor`))
  (`/Engine/EditorBlueprintResources/StandardMacros.IsValid` _returnvalue
    (:`Is Valid`
      (`GameplayStatics.ApplyPointDamage` OtherActor (`self.WeaponDamage`) (- (`self.K2_GetActorLocation` OtherActor) (`self.K2_GetActorLocation` _returnvalue)) SweepResult null _returnvalue "/Script/Engine.DamageType"))))

(fn `UserConstructionScript`)