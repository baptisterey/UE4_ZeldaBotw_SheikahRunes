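; Link's HUD, which creates the gameplay widgets and handles Sheikah rune quick selection.
; BeginPlay caches controller and character, then adds interaction, carry and slate-aim widgets, plus each rune component's own widget class.
; Holding SelectSheikahRune pauses the game and opens a carousel, and releasing applies the selection, unless a Magnesis object is grabbed.
; Axis input scrolls the carousel immediately past a threshold, then repeats after a delay.
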(event `self.ReceiveBeginPlay`
  (set `self.CustomTimeDilation` 1.0)
  (`self.EnableInput` (`self.GetOwningPlayerController`))
  (`|ExecutionSequence`
    (:`then_0`
      ;[0 1 0.3419] Init all the references used by the HUD
      (`|ExecutionSequence`
        (:`then_0`
          (bind _aslink_player_controller (cast `/Game/Blueprints/CharacterLogic/Link_Player_Controller` (`self.GetOwningPlayerController`)))
          (set `self.LinkPlayerController` _aslink_player_controller))
        (:`then_1`
          (bind _aslink_bp (cast `/Game/Blueprints/CharacterLogic/Link_BP` (`Controller.K2_GetPawn` (`self.GetOwningPlayerController`))))
          (set `self.LinkCharacter` _aslink_bp))))
    (:`then_1`
      ;[0 1 0.3419] Create all Widgets used in the game
      (`|ExecutionSequence`
        (:`then_0`
          ;;[1 1 1] InteractWith Widget
          (bind _returnvalue (`|CreateWidget` "/Game/Blueprints/UserInterfaces/InteractionSystem/InteractWith_WBP.InteractWith_WBP_C" (`self.LinkPlayerController`) (`self.LinkCharacter`)))
          (`UserWidget.AddToViewport` _returnvalue 0))
        (:`then_1`
          ;;[1 1 1] CarryableActions Widget
          (bind _returnvalue_2 (`|CreateWidget` "/Game/Blueprints/UserInterfaces/InteractionSystem/Carryable/ManageCarryableActions_WBP.ManageCarryableActions_WBP_C" (`self.LinkPlayerController`) (`self.LinkCharacter`)))
          (`UserWidget.AddToViewport` _returnvalue_2 0))
        (:`then_2`
          ;;[1 1 1] SheikahAim Slate Widget
          (bind _returnvalue_3 (`|CreateWidget` "/Game/Blueprints/UserInterfaces/SheikahSlateAimAction_WBP.SheikahSlateAimAction_WBP_C" (`self.LinkPlayerController`) (`self.LinkCharacter`)))
          (`UserWidget.AddToViewport` _returnvalue_3 0))
        (:`then_3`
          ;;[1 1 1] All Sheikah ActorComponents related Widget
          (for _array_element (`self.K2_GetComponentsByClass` (`self.LinkCharacter`) "/Game/Blueprints/CharacterLogic/SheikahRunes/ActorComponents/SheikahRune_ABP.SheikahRune_ABP_C")
            (bind _returnvalue_4 (`|CreateWidget` (`/Game/Blueprints/CharacterLogic/SheikahRunes/ActorComponents/SheikahRune_ABP.UserWidgetClass` _array_element) (`self.LinkPlayerController`)))
            (bind _assheikah_wbp (cast `/Game/Blueprints/UserInterfaces/SheikahRunes/Sheikah_WBP` _returnvalue_4))
            (`/Game/Blueprints/UserInterfaces/SheikahRunes/Sheikah_WBP.InitSheikahRuneWidget` _assheikah_wbp _array_element (`self.LinkCharacter`))
            (`UserWidget.AddToViewport` _assheikah_wbp 0)))))))

(event `InputAction|SelectSheikahRune` :consume false :paused true
  (params (Key :type "Key Structure"))
  (bind _linkcharacter (`self.LinkCharacter`))
  (bind _sheikahrunes (`/Game/Blueprints/CharacterLogic/Link_BP.GetSheikahRunesInfo` _linkcharacter))
  (bind _returnvalue (not (`KismetSystemLibrary.IsValid` (`/Game/Blueprints/CharacterLogic/Link_BP.GetGrabbedMagnesisObject` (`self.LinkCharacter`)))))
  (:`Pressed`
    (if _returnvalue
      (`/Game/Blueprints/CharacterLogic/Link_Player_Controller.SetGamePaused` (`self.LinkPlayerController`) true)
      (`/Engine/EditorBlueprintResources/StandardMacros.IsValid` (`self.QuickSelectCarouselRef`)
        (:`Is Not Valid`
          (`/Engine/EditorBlueprintResources/StandardMacros.IsValid` (`Controller.K2_GetPawn` (`self.GetOwningPlayerController`))
            (:`Is Valid`
              (bind _returnvalue_2 (`|CreateWidget` "/Game/Blueprints/UserInterfaces/ItemSystem/QuickSelectViaCarousel_WBP.QuickSelectViaCarousel_WBP_C" (`self.GetOwningPlayerController`) _sheikahrunes (`KismetArrayLibrary.Array_Find` _sheikahrunes (`/Game/Blueprints/CharacterLogic/Link_BP.GetCurrentSelectedSheikahRune` _linkcharacter))))
              (bind _output_get (set `self.QuickSelectCarouselRef` _returnvalue_2))
              (`UserWidget.AddToViewport` _output_get 250)))))))
  (:`Released`
    (if _returnvalue
      (`/Game/Blueprints/CharacterLogic/Link_Player_Controller.SetGamePaused` (`self.LinkPlayerController`) false)
      (`/Engine/EditorBlueprintResources/StandardMacros.IsValid` (`self.QuickSelectCarouselRef`)
        (:`Is Valid`
          (`/Engine/EditorBlueprintResources/StandardMacros.IsValid` (`Controller.K2_GetPawn` (`self.GetOwningPlayerController`))
            (:`Is Valid`
              (`/Game/Blueprints/CharacterLogic/Link_BP.SetCurrentSeikahRune` (`self.LinkCharacter`) (`/Game/Blueprints/UserInterfaces/ItemSystem/QuickSelectViaCarousel_WBP.GetSelectedItem` (`self.QuickSelectCarouselRef`)))
              (`Widget.RemoveFromParent` (`self.QuickSelectCarouselRef`))
              (set `self.QuickSelectCarouselRef` null))))))))

(event `InputAxis|QuickSelectNavigation` :consume false :paused true
  (params (AxisValue :type "Float (single-precision)"))
  (set `self.QuickSelectNavigationAxisValue` AxisValue)
  (`/Engine/EditorBlueprintResources/StandardMacros.IsValid` (`self.QuickSelectCarouselRef`)
    (:`Is Valid`
      (if (or (>= (`self.QuickSelectNavigationAxisValue`) (`self.QuickSelectNavigationThreashold`)) (<= (`self.QuickSelectNavigationAxisValue`) (* -1 (`self.QuickSelectNavigationThreashold`))))
        (set `self.TimeSinceQuickSelectChange` (+ (`self.TimeSinceQuickSelectChange`) (`GameplayStatics.GetWorldDeltaSeconds`)))
        (if (or (>= (`self.TimeSinceQuickSelectChange`) (`self.QuickSelectNavigationFirstDelay`)) (== (`self.QuickSelectNavigationNbTimeScroll`) 0))
          (`/Engine/EditorBlueprintResources/StandardMacros.IncrementInt` (`self.QuickSelectNavigationNbTimeScroll`)
            (:`  `
              (set `self.TimeSinceQuickSelectChange` 0.0)
              (`/Game/Blueprints/UserInterfaces/ItemSystem/QuickSelectViaCarousel_WBP.MoveCarousel` (`self.QuickSelectCarouselRef`) (`self.QuickSelectNavigationAxisValue`)))))
        (else
          (set `self.QuickSelectNavigationNbTimeScroll` 0))))))

(fn `UserConstructionScript`)