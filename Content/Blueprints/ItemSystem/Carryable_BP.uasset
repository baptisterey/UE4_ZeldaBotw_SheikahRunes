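; Base carryable item actor that can be grabbed, carried by another actor and dropped as a physics object.
; GrabCarryable disables the mesh's physics and collision, attaches the item to the parent actor and stores a target scene component.
; While carried, Tick uses delta-time lerps to ease relative rotation toward zero and location toward that target plus an offset.
; DropCarryable detaches the item and restores physics and collision.
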(event `self.ReceiveTick`
  (params (DeltaSeconds :type "Float (single-precision)"))
  (if (`self.IsCarryByActor`)
    (`self.K2_SetActorRelativeRotation` (`KismetMathLibrary.RLerp` (`SceneComponent.RelativeRotation` (`self.StaticMesh`)) (struct) (* (`GameplayStatics.GetWorldDeltaSeconds`) (`self.RotateLerpSpeed`))))
    (`/Engine/EditorBlueprintResources/StandardMacros.IsValid` (`self.TargetTransform`)
      (:`Is Valid`
        (`self.K2_SetActorLocation` (`KismetMathLibrary.VLerp` (`self.K2_GetActorLocation`) (+ (`SceneComponent.K2_GetComponentLocation` (`self.TargetTransform`)) (`self.CarryLocationOffset`)) (* (`GameplayStatics.GetWorldDeltaSeconds`) (`self.MoveLerpSpeed`))))))))

(fn `DropCarryable`
  (if (`self.IsCarryByActor`)
    (set `self.IsCarryByActor` false)
    (`PrimitiveComponent.SetSimulatePhysics` (`self.StaticMesh`) true)
    (`PrimitiveComponent.SetCollisionEnabled` (`self.StaticMesh`) "QueryAndPhysics")
    (`self.K2_DetachFromActor` "KeepWorld" "KeepWorld" "KeepWorld")))

(fn `GrabCarryable`
  (params (ParentActor :type "Actor Object Reference") (TargetSceneComponent :type "SceneComponent Object Reference"))
  (`PrimitiveComponent.SetSimulatePhysics` (`self.StaticMesh`) false)
  (`PrimitiveComponent.SetCollisionEnabled` (`self.StaticMesh`) "NoCollision")
  (`self.K2_AttachToActor` (`local.ParentActor`) "None" "KeepWorld" "KeepWorld" "KeepWorld")
  (set `self.IsCarryByActor` true)
  (set `self.TargetTransform` (`local.TargetSceneComponent`)))

(fn `UserConstructionScript`)