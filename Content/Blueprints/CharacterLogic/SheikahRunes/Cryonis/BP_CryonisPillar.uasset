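; BP_CryonisPillar is the pillar actor for the Cryonis Sheikah rune.
; On BeginPlay a timeline grows the mesh along its Z scale while a pillar particle effect spawns.
; A dynamic material created at construction lets Select and Unselect raise or restore emission to show highlighting.
; On destruction it deactivates the stored effect and spawns a destruction effect at the pillar's middle point.
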(event `self.ReceiveBeginPlay`
  (bind (_returnvalue_location _returnvalue_rotation _returnvalue_scale) (`KismetMathLibrary.BreakTransform` (`self.GetTransform`)))
  (`|ExecutionSequence`
    (:`then_0`
      (bind (_direction _scalezvalue) (`Timeline|SpawnAnimation`)
        (:`Update`
          (`SceneComponent.SetRelativeScale3D` (`self.PillarMesh`) (`KismetMathLibrary.MakeVector` 1.0 1.0 _scalezvalue)))
        (:`Finished`
          (`ActorComponent.Deactivate` (`self.CreateParticleSystem`)))))
    (:`then_1`
      (bind _returnvalue (`GameplayStatics.SpawnEmitterAtLocation` "/Game/VFXs/SheikahRunes/Cryonis/VFX_Cryonis_Pillar.VFX_Cryonis_Pillar" (+ _returnvalue_location (* (`self.GetActorUpVector`) (0.0 0.0 150.0))) _returnvalue_rotation _returnvalue_scale))
      (set `self.PillarFxRef` _returnvalue))))

(event `/Game/Blueprints/Interfaces/BPI_Selectable.Select`
  (`MaterialInstanceDynamic.SetScalarParameterValue` (`self.PillarDynamicMaterialInstance`) "EmissionAmplitude" 3.0))

(event `/Game/Blueprints/Interfaces/BPI_Selectable.Unselect`
  (`MaterialInstanceDynamic.SetScalarParameterValue` (`self.PillarDynamicMaterialInstance`) "EmissionAmplitude" 1.0))

(event `self.ReceiveDestroyed`
  (`ActorComponent.Deactivate` (`self.PillarFxRef`))
  (`GameplayStatics.SpawnEmitterAtLocation` "/Game/VFXs/SheikahRunes/Cryonis/VFX_Cryonis_PillarDestroyed.VFX_Cryonis_PillarDestroyed" (`SceneComponent.K2_GetComponentLocation` (`self.MiddlePillarPoint`))))

(fn `UserConstructionScript`
  (bind _pillarmesh (`self.PillarMesh`))
  (bind _returnvalue (`PrimitiveComponent.CreateDynamicMaterialInstance` _pillarmesh 0 (`PrimitiveComponent.GetMaterial` _pillarmesh 0) "None"))
  (set `self.PillarDynamicMaterialInstance` _returnvalue))