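; Placement preview for the Cryonis rune that shows whether the space it occupies is free.
; Box overlap events track the actors inside and update the free-space flag, which fires a dispatcher only when it changes.
; When free, a timeline animates the preview box's Z scale and a dynamic material sets its blinking state.
; When blocked, the animation stops, the box flattens and the blinking state inverts.
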(event `self.ReceiveBeginPlay`
  (`parent.ReceiveBeginPlay`)
  (add `self.IsSpaceFreeChangedEvent` (delegate `IsSpaceFreeChangedEvent_Event`))
  (`MaterialInstanceDynamic.SetScalarParameterValue` (`self.PreviewBoxMaterialInstance`) "BlinkingState" 1.0 :!label _label)
  (bind (_direction _zscalevalue) (`Timeline|PreviewAnimation` :!via `PlayFromStart` :!label _label_2)
    (:`Update`
      (`SceneComponent.SetRelativeScale3D` (`self.PreviewBox`) (`KismetMathLibrary.MakeVector` 1.0 1.0 _zscalevalue)))))

(event `IsSpaceFreeChangedEvent_Event` :!signature `self.IsSpaceFreeChangedEvent`
  (params (IsSpaceFree :type Boolean))
  (if (`self.IsSpaceFree`)
    (goto _label)
    (else
      (`SceneComponent.SetRelativeScale3D` (`self.PreviewBox`) (1.0 1.0 0.1))
      (`|ExecutionSequence`
        (:`then_0`
          (goto _label_2 :!via `Stop`))
        (:`then_1`
          (`MaterialInstanceDynamic.SetScalarParameterValue` (`self.PreviewBoxMaterialInstance`) "BlinkingState" -1.0))))))

(event `self.Box.OnComponentBeginOverlap`
  (params (OverlappedComponent :type "PrimitiveComponent Object Reference") (OtherActor :type "Actor Object Reference") (OtherComp :type "PrimitiveComponent Object Reference") (OtherBodyIndex :type Integer) (bFromSweep :type Boolean) (SweepResult :type "HitResult Structure (by ref)"))
  ;[1 0 0] Preview Hitboxes Overlap Events
  (`KismetArrayLibrary.Array_Add` (`self.ActorsInsidePreviewBox`) OtherActor)
  (if (>= (`KismetArrayLibrary.Array_Length` (`self.ActorsInsidePreviewBox`)) 1)
    (`self.SetIsSpaceFree` false)))

(event `self.Box.OnComponentEndOverlap`
  (params (OverlappedComponent :type "PrimitiveComponent Object Reference") (OtherActor :type "Actor Object Reference") (OtherComp :type "PrimitiveComponent Object Reference") (OtherBodyIndex :type Integer))
  ;[1 0 0] Preview Hitboxes Overlap Events
  (`KismetArrayLibrary.Array_RemoveItem` (`self.ActorsInsidePreviewBox`) OtherActor)
  (if (== (`KismetArrayLibrary.Array_Length` (`self.ActorsInsidePreviewBox`)) 0)
    (`self.SetIsSpaceFree` true)))

(fn `SetIsSpaceFree`
  (params (`New Value` :type Boolean))
  (if (!= `New Value` (`self.IsSpaceFree`))
    (bind _output_get (set `self.IsSpaceFree` `New Value`))
    (`self.IsSpaceFreeChangedEvent` _output_get)))

(fn `SpaceFree`
  (returns (IsSpaceFree :type Boolean))
  (return (`self.IsSpaceFree`)))

(fn `UserConstructionScript`
  (bind _previewbox (`self.PreviewBox`))
  (bind _returnvalue (`PrimitiveComponent.CreateDynamicMaterialInstance` _previewbox 0 (`PrimitiveComponent.GetMaterial` _previewbox 0) "None"))
  (set `self.PreviewBoxMaterialInstance` _returnvalue))