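; BP_CheckMagnesisSphere is a moving probe that looks for an object to target with the Magnesis rune.
; Each tick it moves along its forward vector without sweeping, measuring its distance from LinkRef.
; The first overlap with an actor other than LinkRef, or reaching max range, fires OnCheckMagnesisSphereFindObject with that actor or none, then destroys the sphere.
; It does not filter for magnetic objects itself.
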(event `self.ReceiveTick`
  (params (DeltaSeconds :type "Float (single-precision)"))
  ;[1 1 1] Move along forward vector
  (`self.K2_SetActorLocation` (+ (`self.K2_GetActorLocation`) (* (`self.GetActorForwardVector`) (* (`self.MoveSpeed`) (`GameplayStatics.GetWorldDeltaSeconds`)))))
  ;[1 1 1] Check Max Distance
  (if (>= (`KismetMathLibrary.Vector_Distance` (`self.K2_GetActorLocation` (`self.LinkRef`)) (`self.K2_GetActorLocation`)) (`self.SphereMaxRange`))
    (`self.OnCheckMagnesisSphereFindObject` null)
    (`self.K2_DestroyActor`)))

(event `self.Sphere.OnComponentBeginOverlap`
  (params (OverlappedComponent :type "PrimitiveComponent Object Reference") (OtherActor :type "Actor Object Reference") (OtherComp :type "PrimitiveComponent Object Reference") (OtherBodyIndex :type Integer) (bFromSweep :type Boolean) (SweepResult :type "HitResult Structure (by ref)"))
  (if (!= OtherActor (`self.LinkRef`))
    (`self.OnCheckMagnesisSphereFindObject` OtherActor)
    (`self.K2_DestroyActor`)))

(fn `UserConstructionScript`)