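; BP_MagnesisMagnet is the magnet visual actor for the Magnesis rune, showing a mesh with two particle beams.
; On BeginPlay it hides the mesh and both particle systems, then reveals them after a brief timer delay.
; SetBeamTargetLocation aims both beams at a given point, offsetting each sideways along the actor's right vector in opposite directions so they end side by side.
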(event `self.ReceiveBeginPlay`
  (`SceneComponent.SetVisibility` (`self.StaticMesh`) false true)
  (`SceneComponent.SetVisibility` (`self.ParticleSystem1`) false true)
  (`SceneComponent.SetVisibility` (`self.ParticleSystem`) false true)
  (`KismetSystemLibrary.K2_SetTimerDelegate` (delegate `OnInitialWaitEnd`) 0.05))

(event `OnInitialWaitEnd`
  (`SceneComponent.SetVisibility` (`self.StaticMesh`) true true)
  (`SceneComponent.SetVisibility` (`self.ParticleSystem1`) true true)
  (`SceneComponent.SetVisibility` (`self.ParticleSystem`) true true))

(fn `SetBeamTargetLocation`
  (params (NewTargetPoint :type "Vector Structure"))
  (`ParticleSystemComponent.SetBeamTargetPoint` (`self.ParticleSystem1`) 0 (+ NewTargetPoint (* (`KismetMathLibrary.GetRightVector` (`self.K2_GetActorRotation`)) -15.0)) 0)
  (`ParticleSystemComponent.SetBeamTargetPoint` (`self.ParticleSystem`) 0 (+ (`local.NewTargetPoint`) (* (`KismetMathLibrary.GetRightVector` (`self.K2_GetActorRotation`)) 15.0)) 0))

(fn `UserConstructionScript`)