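; Base actor component for Link's Sheikah runes, providing shared references, a cooldown and empty input events for runes to implement.
; On BeginPlay it caches the owning Link_BP and its player camera manager.
; StartCoolDown runs a timer and signals cooldown changes, while Tick accumulates elapsed time so GetRemainingCooldownTime can return a clamped remaining fraction.
; The Sheikah and main action events receive a rune instance but have no logic here.
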(event `self.ReceiveBeginPlay`
  (bind _aslink_bp (cast `/Game/Blueprints/CharacterLogic/Link_BP` (`self.GetOwner`)))
  (bind _output_get (set `self.LinkRef` _aslink_bp))
  (bind _asplayer_controller (cast `PlayerController` (`Pawn.GetController` _output_get)))
  (set `self.CameraManagerRef` (`PlayerController.PlayerCameraManager` _asplayer_controller)))

(event `self.ReceiveTick`
  (params (DeltaSeconds :type "Float (single-precision)"))
  (if (`self.IsInCooldown`)
    (set `self.TimeInCoolDown` (+ (`self.TimeInCoolDown`) (`GameplayStatics.GetWorldDeltaSeconds`)))))

(event `StartCoolDown`
  (if (not (`self.IsInCooldown`))
    (set `self.IsInCooldown` true)
    (`KismetSystemLibrary.K2_SetTimerDelegate` (delegate `OnCooldownOver`) (`self.CoolDownTime`))
    (set `self.TimeInCoolDown` 0.0)
    (`self.OnCooldownChanged` true)))

(event `OnCooldownOver`
  (set `self.IsInCooldown` false)
  (`self.OnCooldownChanged` false))

(event `OnSheikahActionPressed`
  (params (SheikahRuneInstance :type "/Game/Blueprints/ItemSystem/DataStructures/ItemInstance Object Reference")))

(event `OnSheikahActionReleased`
  (params (SheikahRuneInstance :type "/Game/Blueprints/ItemSystem/DataStructures/ItemInstance Object Reference")))

(event `OnMainActionPressed`
  (params (SheikahRuneInstance :type "/Game/Blueprints/ItemSystem/DataStructures/ItemInstance Object Reference")))

(fn `Get Remaining Cooldown Time`
  (returns (TimeRemaining :type "Float (double-precision)"))
  (return (`KismetMathLibrary.FClamp` (- 1.0 (/ (`self.TimeInCoolDown`) (`self.CoolDownTime`))))))