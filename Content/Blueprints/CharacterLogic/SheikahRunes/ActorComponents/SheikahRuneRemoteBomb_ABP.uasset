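; Actor component for the Sheikah Remote Bomb rune, letting Link spawn a bomb and detonate it with the same action press.
; With no valid bomb and Link's hands free, a press spawns one at his spawn point and has him grab it as a carryable.
; While that bomb exists, a press explodes it unless it is still being carried; releasing the action does nothing.
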(event `self.OnSheikahActionPressed`
  (params (SheikahRuneInstance :type "/Game/Blueprints/ItemSystem/DataStructures/ItemInstance Object Reference"))
  (`/Engine/EditorBlueprintResources/StandardMacros.IsValid` (`self.RemoteBombRef`)
    (:`Is Valid`
      (if (not (`/Game/Blueprints/ItemSystem/Carryable_BP.Is Carry by Actor` (`self.RemoteBombRef`)))
        (`/Game/Blueprints/CharacterLogic/SheikahRunes/RemoteBomb_BP.ExplodeBomb` (`self.RemoteBombRef`))))
    (:`Is Not Valid`
      (if (not (`/Game/Blueprints/CharacterLogic/Link_BP.IsCarryingActor` (`self.LinkRef`)))
        (bind _returnvalue (`|SpawnActorFromClass` (`self.RemoteBombToSpawn`) (`KismetMathLibrary.MakeTransform` (`SceneComponent.K2_GetComponentLocation` (`/Game/Blueprints/CharacterLogic/Link_BP.SpawnRemoteBombPoint` (`self.LinkRef`))) (`Actor.K2_GetActorRotation` (`self.LinkRef`))) "AlwaysSpawn" "OverrideRootScale" null (`self.LinkRef`)))
        (set `self.RemoteBombRef` _returnvalue)
        (`/Game/Blueprints/CharacterLogic/Link_BP.GrabCarryable` (`self.LinkRef`) _returnvalue)))))

(event `self.OnSheikahActionReleased`
  (params (SheikahRuneInstance :type "/Game/Blueprints/ItemSystem/DataStructures/ItemInstance Object Reference")))