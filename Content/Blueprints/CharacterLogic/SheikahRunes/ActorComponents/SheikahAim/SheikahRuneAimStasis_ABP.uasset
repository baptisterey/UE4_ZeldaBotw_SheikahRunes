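; Actor component for the Stasis Sheikah rune aim, letting Link freeze one object at a time and launch it.
; Trace results select actors carrying a stasis component and update the interaction state for the UI.
; The main action freezes the selected actor, or launches it if already frozen, then toggles aim off.
; It binds to the frozen component's launch event, by player or timer, to clear the reference and start cooldown.
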(event `self.OnMainActionPressed`
  (params (SheikahRuneInstance :type "/Game/Blueprints/ItemSystem/DataStructures/ItemInstance Object Reference"))
  (bind _returnvalue (`Actor.GetComponentByClass` (`self.GetCurrentSelectedActor`) "/Game/Blueprints/CharacterLogic/SheikahRunes/Stasis/ABP_StasisComponent.ABP_StasisComponent_C"))
  (`/Engine/EditorBlueprintResources/StandardMacros.IsValid` (`self.GetCurrentSelectedActor`)
    (:`Is Valid`
      (`/Engine/EditorBlueprintResources/StandardMacros.IsValid` (`self.CurrentFrozenObject`)
        (:`Is Valid`
          ;[1 0 0.04918] Trying to launch the currently frozen object
          (if (== (`self.GetOwner` (`self.CurrentFrozenObject`)) (`self.GetCurrentSelectedActor`))
            (`/Game/Blueprints/CharacterLogic/SheikahRunes/Stasis/ABP_StasisComponent.LaunchStatis` (`self.CurrentFrozenObject`))
            (`/Game/Blueprints/CharacterLogic/Link_BP.PlaySheikahSlateAnimation` (`self.LinkRef`) :!label _label)
            (`/Game/Blueprints/CharacterLogic/Link_BP.Toggle Sheikah Aim` (`self.LinkRef`) "NewEnumerator3")))
        (:`Is Not Valid`
          (`/Engine/EditorBlueprintResources/StandardMacros.IsValid` _returnvalue
            (:`Is Valid`
              (set `self.CurrentFrozenObject` _returnvalue)
              (`/Game/Blueprints/CharacterLogic/SheikahRunes/Stasis/ABP_StasisComponent.ActiveStatisPower` (`self.CurrentFrozenObject`))
              (add `/Game/Blueprints/CharacterLogic/SheikahRunes/Stasis/ABP_StasisComponent.OnLaunchedStasis` (`self.CurrentFrozenObject`) (delegate `OnCurrentFrozenObjectLaunch`))
              (goto _label))))))
    (:`Is Not Valid`
      (`/Game/Blueprints/CharacterLogic/Link_BP.PlaySheikahSlateAnimation` (`self.LinkRef`)))))

(event `OnCurrentFrozenObjectLaunch`
  ;[1 1 1] Bind on Frozen object to know when it launches, can be because of Link or because of timer
  (remove `/Game/Blueprints/CharacterLogic/SheikahRunes/Stasis/ABP_StasisComponent.OnLaunchedStasis` (`self.CurrentFrozenObject`) (delegate `OnCurrentFrozenObjectLaunch`))
  (set `self.CurrentFrozenObject` null)
  (`self.StartCoolDown`))

(event `self.OnTraceLineResult`
  (params (HitResult :type "HitResult Structure (by ref)") (HasHit :type Boolean))
  (bind (_bblockinghit _binitialoverlap _time _distance _location _impactpoint _normal _impactnormal _physmat _hitactor) (`GameplayStatics.BreakHitResult` HitResult))
  (`|ExecutionSequence`
    (:`then_0`
      (if HasHit
        (`/Engine/EditorBlueprintResources/StandardMacros.IsValid` (`Actor.GetComponentByClass` _hitactor "/Game/Blueprints/CharacterLogic/SheikahRunes/Stasis/ABP_StasisComponent.ABP_StasisComponent_C")
          (:`Is Valid`
            (`self.SetCurrentSelectedActor` _hitactor))
          (:`Is Not Valid`
            (`self.SetCurrentSelectedActor` null)))
        (else
          (`self.SetCurrentSelectedActor` null))))
    (:`then_1`
      (`self.Manage New Interaction Possible`))))

(event `self.OnLookingForTargetChanged`
  (params (NewValue :type Boolean))
  (`parent.OnLookingForTargetChanged` NewValue)
  (if (not NewValue)
    (`|ExecutionSequence`
      (:`then_0`
        ;[1 1 1] Reset the selected object
        (`self.SetCurrentSelectedActor` null))
      (:`then_1`
        ;[1 1 1] Calling event for UI
        (`self.SetInteractionPossible` "NewEnumerator0")))))

(fn `Has Frozen Object`
  (returns (Value :type Boolean))
  (return (`KismetSystemLibrary.IsValid` (`self.CurrentFrozenObject`))))

(fn `Manage New Interaction Possible`
  (bind _returnvalue (`KismetSystemLibrary.IsValid` (`self.GetCurrentSelectedActor`)))
  (if (and (`KismetSystemLibrary.IsValid` (`self.GetCurrentSelectedActor`)) (not (`KismetSystemLibrary.IsValid` (`self.CurrentFrozenObject`))))
    (`self.SetInteractionPossible` "NewEnumerator5")
    (else
      (`/Engine/EditorBlueprintResources/StandardMacros.IsValid` (`self.CurrentFrozenObject`)
        (:`Is Valid`
          (if (and _returnvalue (== (`self.GetCurrentSelectedActor`) (`self.GetOwner` (`self.CurrentFrozenObject`))))
            (`self.SetInteractionPossible` "NewEnumerator6")
            (elif _returnvalue
              (`self.SetInteractionPossible` "NewEnumerator8")
              (else
                (`self.SetInteractionPossible` "NewEnumerator1" :!label _label)))))
        (:`Is Not Valid`
          (goto _label))))))