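; Magnesis rune aim component that picks a magnetic target and launches the Magnesis orb at it.
; Trace results select the hit actor only if it has a Magnesis component, otherwise they clear the selection.
; The main action passes the selected actor to LinkRef to launch the orb.
; When target search stops, it runs parent logic, clears the selection and updates the interaction state for the UI.
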(event `self.OnMainActionPressed`
  (params (SheikahRuneInstance :type "/Game/Blueprints/ItemSystem/DataStructures/ItemInstance Object Reference"))
  (`/Game/Blueprints/CharacterLogic/Link_BP.LaunchMagnesisOrb` (`self.LinkRef`) (`self.GetCurrentSelectedActor`)))

(event `self.OnTraceLineResult`
  (params (HitResult :type "HitResult Structure (by ref)") (HasHit :type Boolean))
  (bind (_bblockinghit _binitialoverlap _time _distance _location _impactpoint _normal _impactnormal _physmat _hitactor) (`GameplayStatics.BreakHitResult` HitResult))
  (`|ExecutionSequence`
    (:`then_0`
      ;[1 1 1] Manage Trace
      (if HasHit
        (`/Engine/EditorBlueprintResources/StandardMacros.IsValid` (`Actor.GetComponentByClass` _hitactor "/Game/Blueprints/CharacterLogic/SheikahRunes/Magnesis/ABP_MagnesisComponent.ABP_MagnesisComponent_C")
          (:`Is Valid`
            (`self.SetCurrentSelectedActor` _hitactor))
          (:`Is Not Valid`
            (`self.SetCurrentSelectedActor` null)))
        (else
          (`self.SetCurrentSelectedActor` null))))))

(event `self.OnLookingForTargetChanged`
  (params (NewValue :type Boolean))
  (`parent.OnLookingForTargetChanged` NewValue)
  (if (not NewValue)
    (`|ExecutionSequence`
      (:`then_0`
        ;[1 1 1] Reset the selected object
        (`self.SetCurrentSelectedActor` null))
      (:`then_1`
        ;[1 1 1] Calling event for UI
        (`self.SetInteractionPossible` "NewEnumerator0")))))