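; Aim component for the Cryonis Sheikah rune, letting the player place ice pillars on water or destroy existing ones.
; Trace results on water move a preview cube, oriented by a normal dot-up test for flat or vertical surfaces; elsewhere they select any pillar hit.
; The main action spawns a pillar at a free preview, evicting the oldest at the limit and starting cooldown, or destroys the selection.
; Preview and selection changes drive UI interaction events.
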(event `self.OnMainActionPressed`
  (params (SheikahRuneInstance :type "/Game/Blueprints/ItemSystem/DataStructures/ItemInstance Object Reference"))
  (`/Engine/EditorBlueprintResources/StandardMacros.IsValid` (`self.CubePreviewRef`)
    (:`Is Valid`
      (if (and (`/Game/Blueprints/CharacterLogic/SheikahRunes/Cryonis/BP_CryonisPreview.SpaceFree` (`self.CubePreviewRef`)) (not (`self.IsInCooldown`)))
        ;[1 1 1] Create a new Cryonis pillar
        (if (>= (`KismetArrayLibrary.Array_Length` (`self.CryonisPillars`)) (`self.MaxCryonisPillars`))
          ;;[1 0 0] Destroy the oldset pillar as we reached our limit
          (`Actor.K2_DestroyActor` (`|GetArrayItem` (`self.CryonisPillars`)))
          (`KismetArrayLibrary.Array_Remove` (`self.CryonisPillars`)))
        ;;[0.162 1 0] Spawn a new pillar
        (bind _returnvalue (`|SpawnActorFromClass` "/Game/Blueprints/CharacterLogic/SheikahRunes/Cryonis/BP_CryonisPillar.BP_CryonisPillar_C" (`Actor.GetTransform` (`self.CubePreviewRef`)) "Undefined" "OverrideRootScale" null null))
        (`KismetArrayLibrary.Array_Add` (`self.CryonisPillars`) _returnvalue)
        ;;[0.04102 1 0] Destroy the preview pillar as we enter cooldown
        (`Actor.K2_DestroyActor` (`self.CubePreviewRef`))
        ;[1 0.4397 0] Cryonis used : Start the cooldown
        (`self.StartCoolDown`)
        ;[1 0.4397 0] Cryonis Used : Leave the aiming state and play the right animation
        (`/Game/Blueprints/CharacterLogic/Link_BP.Toggle Sheikah Aim` (`self.LinkRef`) "NewEnumerator3")
        (`/Game/Blueprints/CharacterLogic/Link_BP.PlaySheikahSlateAnimation` (`self.LinkRef`))))
    (:`Is Not Valid`
      (`/Engine/EditorBlueprintResources/StandardMacros.IsValid` (`self.GetCurrentSelectedActor`)
        (:`Is Valid`
          ;[1 1 1] Destroy the current selected pillar
          (`KismetArrayLibrary.Array_RemoveItem` (`self.CryonisPillars`) (`self.GetCurrentSelectedActor`))
          (`Actor.K2_DestroyActor` (`self.GetCurrentSelectedActor`))
          (`/Game/Blueprints/CharacterLogic/Link_BP.PlaySheikahSlateAnimation` (`self.LinkRef`))
          ;[1 1 1] If it was the last pillar, leave the Aiming State
          (if (== (`KismetArrayLibrary.Array_Length` (`self.CryonisPillars`)) 0)
            (`/Game/Blueprints/CharacterLogic/Link_BP.Toggle Sheikah Aim` (`self.LinkRef`) "NewEnumerator3")))))))

(event `OnCubePreviewSpaceFreeChanged`
  (params (IsSpaceFree :type Boolean))
  (if IsSpaceFree
    (`self.OnInteractionPossibleChanged` "NewEnumerator2")
    (else
      (`self.OnInteractionPossibleChanged` "NewEnumerator4"))))

(event `self.OnTraceLineResult`
  (params (HitResult :type "HitResult Structure (by ref)") (HasHit :type Boolean))
  (bind _cubepreviewref (`self.CubePreviewRef`))
  (bind (_cubepreviewtransform_location _cubepreviewtransform_rotation) (`KismetMathLibrary.BreakTransform` (`self.CubePreviewTransform`)))
  (bind (_bblockinghit _binitialoverlap _time _distance _location _impactpoint _normal _impactnormal) (`GameplayStatics.BreakHitResult` (`self.HitResult`)))
  (bind (_bblockinghit_2 _binitialoverlap_2 _time_2 _distance_2 _location_2) (`GameplayStatics.BreakHitResult` (`self.HitResult`)))
  (bind (_bblockinghit_3 _binitialoverlap_3 _time_3 _distance_3 _location_3 _impactpoint_2 _normal_2 _impactnormal_2 _physmat _hitactor) (`GameplayStatics.BreakHitResult` (`self.HitResult`)))
  (bind (_returnvalue_roll _returnvalue_pitch _returnvalue_yaw) (`KismetMathLibrary.BreakRotator` (`KismetMathLibrary.FindLookAtRotation` _location_2 (`Actor.K2_GetActorLocation` (`self.GetOwner`)))))
  (bind (_returnvalue_roll_2 _returnvalue_pitch_2) (`KismetMathLibrary.BreakRotator` (`KismetMathLibrary.Conv_VectorToRotator` _location_2)))
  (bind (_returnvalue_roll_3 _returnvalue_pitch_3 _returnvalue_yaw_2) (`KismetMathLibrary.BreakRotator` (`KismetMathLibrary.Conv_VectorToRotator` _impactnormal)))
  (set `self.HitResult` HitResult)
  (set `self.HasHit` HasHit)
  (set `self.DestroyedCubePreview` false)
  (set `self.PreviousCubePreviewRef` (`self.CubePreviewRef`))
  (set `self.PreviousSelectedPillarRef` (`self.GetCurrentSelectedActor`))
  (`|ExecutionSequence`
    (:`then_0`
      (if (`self.HasHit`)
        (if (`|EnumEquality` (`PrimitiveComponent.GetCollisionObjectType` (`.HitComponent` (`GameplayStatics.BreakHitResult` (`self.HitResult`)))) "ECC_GameTraceChannel3")
          (`self.SetCurrentSelectedActor` null)
          (if (> (`KismetMathLibrary.Dot_VectorVector` (0.0 0.0 1.0) (`.ImpactNormal` (`GameplayStatics.BreakHitResult` (`self.HitResult`)))) 0.5)
            (set `self.CubePreviewTransform` (`KismetMathLibrary.MakeTransform` _location_2 (`KismetMathLibrary.MakeRotator` _returnvalue_roll_2 _returnvalue_pitch_2 _returnvalue_yaw)))
            (else
              (set `self.CubePreviewTransform` (`KismetMathLibrary.MakeTransform` _location (`KismetMathLibrary.MakeRotator` _returnvalue_roll_3 (+ _returnvalue_pitch_3 -90.0) _returnvalue_yaw_2)))))
          (`/Engine/EditorBlueprintResources/StandardMacros.IsValid` (`self.CubePreviewRef`)
            (:`Is Valid`
              (`Actor.K2_SetActorLocationAndRotation` (`self.CubePreviewRef`) _cubepreviewtransform_location _cubepreviewtransform_rotation false false))
            (:`Is Not Valid`
              (bind _returnvalue (`|SpawnActorFromClass` "/Game/Blueprints/CharacterLogic/SheikahRunes/Cryonis/BP_CryonisPreview.BP_CryonisPreview_C" (`self.CubePreviewTransform`) "Undefined" "OverrideRootScale" (`self.GetOwner`) null))
              (bind _output_get (set `self.CubePreviewRef` _returnvalue))
              (add `/Game/Blueprints/CharacterLogic/SheikahRunes/Cryonis/BP_CryonisPreview.IsSpaceFreeChangedEvent` _output_get (delegate `OnCubePreviewSpaceFreeChanged`))))
          (else
            (`|ExecutionSequence` :!label _label
              (:`then_0`
                (`/Engine/EditorBlueprintResources/StandardMacros.IsValid` _cubepreviewref
                  (:`Is Valid`
                    (clear `/Game/Blueprints/CharacterLogic/SheikahRunes/Cryonis/BP_CryonisPreview.IsSpaceFreeChangedEvent` _cubepreviewref)
                    (`Actor.K2_DestroyActor` _cubepreviewref)
                    (set `self.CubePreviewRef` null)
                    (set `self.DestroyedCubePreview` true))))
              (:`then_1`
                (`self.SetCurrentSelectedActor` null)
                (if _bblockinghit_3
                  (bind _asbp_cryonis_pillar (cast `/Game/Blueprints/CharacterLogic/SheikahRunes/Cryonis/BP_CryonisPillar` _hitactor))
                  (`self.SetCurrentSelectedActor` _asbp_cryonis_pillar))))))
        (else
          (goto _label))))
    (:`then_1`
      (if (!= (`self.PreviousCubePreviewRef`) (`self.CubePreviewRef`))
        (if (`KismetSystemLibrary.IsValid` (`self.CubePreviewRef`))
          (if (`/Game/Blueprints/CharacterLogic/SheikahRunes/Cryonis/BP_CryonisPreview.SpaceFree` (`self.CubePreviewRef`))
            (`self.OnInteractionPossibleChanged` "NewEnumerator2")
            (else
              (`self.OnInteractionPossibleChanged` "NewEnumerator4")))
          (else
            (if (!= (`self.PreviousSelectedPillarRef`) (`self.GetCurrentSelectedActor`)) :!label _label_2
              (if (`KismetSystemLibrary.IsValid` (`self.GetCurrentSelectedActor`))
                (`self.OnInteractionPossibleChanged` "NewEnumerator3")
                (else
                  (`self.OnInteractionPossibleChanged` "NewEnumerator1")))
              (elif (`self.DestroyedCubePreview`)
                (`self.OnInteractionPossibleChanged` "NewEnumerator1")))))
        (else
          (goto _label_2))))))

(event `self.OnLookingForTargetChanged`
  (params (NewValue :type Boolean))
  (`parent.OnLookingForTargetChanged` NewValue)
  (if (not NewValue)
    (`|ExecutionSequence`
      (:`then_0`
        ;[1 1 1] We are no longer casting trace, destroy the preview cube if any
        (`/Engine/EditorBlueprintResources/StandardMacros.IsValid` (`self.CubePreviewRef`)
          (:`Is Valid`
            (`Actor.K2_DestroyActor` (`self.CubePreviewRef`)))))
      (:`then_1`
        ;[1 1 1] Reset the selected pillar
        (`self.SetCurrentSelectedActor` null))
      (:`then_2`
        ;[1 1 1] Calling event for UI
        (`self.OnInteractionPossibleChanged` "NewEnumerator0")))))