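; Remote Bomb Sheikah rune actor: a carryable bomb that plays a sound on spawn and explodes in a radial blast.
; Taking radial damage triggers ExplodeBomb, which makes any carrier drop it, destroys the actor and deals full, non-diminishing damage within its radius.
; The blast spawns explosion VFX, then loops over all player controllers, playing a camera shake and spawning the explosion sound once per controller.
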(event `self.ReceiveBeginPlay`
  (`parent.ReceiveBeginPlay`)
  (`GameplayStatics.PlaySoundAtLocation` (`self.CreateSound`) (`self.K2_GetActorLocation`) (struct) 1.0 1.0 0.0 "/Game/Sounds/SheikahSlate/RemoteBomb/Attenuation_RemoteBombExplode.Attenuation_RemoteBombExplode" null null))

(event `self.ReceiveTick`
  (params (DeltaSeconds :type "Float (single-precision)"))
  (`parent.ReceiveTick` DeltaSeconds))

(event `self.ReceiveRadialDamage`
  (params (DamageReceived :type "Float (single-precision)") (DamageType :type "DamageType Object Reference") (Origin :type "Vector Structure") (HitInfo :type "HitResult Structure (by ref)") (InstigatedBy :type "Controller Object Reference") (DamageCauser :type "Actor Object Reference"))
  (`self.ExplodeBomb`))

(fn `ExplodeBomb`
  (bind _damageradius (`self.DamageRadius`))
  (bind _basedamage (`self.BaseDamage`))
  (if (`self.Is Carry by Actor`)
    (`/Game/Blueprints/CharacterLogic/Link_BP.DropCurrentCarryable` (`self.CarryingActor`) true))
  (`self.K2_DestroyActor`)
  (`GameplayStatics.ApplyRadialDamageWithFalloff` :`BaseDamage` _basedamage :`MinimumDamage` _basedamage :`Origin` (`self.K2_GetActorLocation`) :`DamageInnerRadius` _damageradius :`DamageOuterRadius` _damageradius :`DamageTypeClass` "/Game/Blueprints/DamageTypes/SheikahBombDamageType.SheikahBombDamageType_C" :`DamageCauser` self :`InstigatedByController` (`Pawn.GetController` (`self.Instigator`)))
  (`GameplayStatics.SpawnEmitterAtLocation` "/Game/VFXs/SheikahRunes/RemoteBombs/VFX_RemoteBombExplosion.VFX_RemoteBombExplosion" (`self.K2_GetActorLocation`))
  (bind _outactors (`GameplayStatics.GetAllActorsOfClass` "/Script/Engine.PlayerController"))
  (for _array_element _outactors
    (`PlayerController.ClientStartCameraShake` :`self` _array_element :`Shake` "/Game/Data/RemoteBomb_CameraShake.RemoteBomb_CameraShake_C")
    (`GameplayStatics.SpawnSoundAtLocation` (`self.ExplosionSound`) (`self.K2_GetActorLocation`) (struct) 1.25 1.0 0.0 "/Game/Sounds/SheikahSlate/RemoteBomb/Attenuation_RemoteBombExplode.Attenuation_RemoteBombExplode" null)))

(fn `UserConstructionScript`)